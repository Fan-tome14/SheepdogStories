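; BP_Enclos is a sheep enclosure that tracks a count toward a win condition, shown only as printed text.
; On BeginPlay it reads the target total from the MassSheepManager's NumberOfSheep.
; Box overlap begin and end events raise and lower the count, filtering on a cast to MassSheepManager itself rather than a sheep class.
; Reaching the total on entry prints "gagner !"; otherwise the current count prints.
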(event `self.ReceiveBeginPlay`
  (bind _returnvalue (`GameplayStatics.GetActorOfClass` "/Script/SheepdogStories.MassSheepManager"))
  (bind _output_get (set `self.totalSheepCount` (`MassSheepManager.NumberOfSheep` _returnvalue)))
  (`KismetSystemLibrary.PrintText` (`KismetTextLibrary.Conv_IntToText` _output_get)))

(event `self.ReceiveTick`
  (params (DeltaSeconds :type "Float (single-precision)")))

(event `self.Box.OnComponentBeginOverlap`
  (params (OverlappedComponent :type "PrimitiveComponent Object Reference") (OtherActor :type "Actor Object Reference") (OtherComp :type "PrimitiveComponent Object Reference") (OtherBodyIndex :type Integer) (bFromSweep :type Boolean) (SweepResult :type "HitResult Structure (by ref)"))
  (cast `MassSheepManager` OtherActor)
  (set `self.SheepInEnclosure` (+ (`self.SheepInEnclosure`) 1))
  (if (>= (`self.SheepInEnclosure`) (`self.totalSheepCount`))
    (`KismetSystemLibrary.PrintText` "gagner !")
    (else
      (`KismetSystemLibrary.PrintText` (`KismetTextLibrary.Conv_IntToText` (`self.SheepInEnclosure`))))))

(event `self.Box.OnComponentEndOverlap`
  (params (OverlappedComponent :type "PrimitiveComponent Object Reference") (OtherActor :type "Actor Object Reference") (OtherComp :type "PrimitiveComponent Object Reference") (OtherBodyIndex :type Integer))
  (cast `MassSheepManager` OtherActor)
  (set `self.SheepInEnclosure` (- (`self.SheepInEnclosure`) 1))
  (`KismetSystemLibrary.PrintText` (`KismetTextLibrary.Conv_IntToText` (`self.SheepInEnclosure`))))

(fn `UserConstructionScript`)