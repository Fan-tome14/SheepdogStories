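; BP_EnclosV2 is the sheep enclosure goal that detects when the flocking minigame is won.
; On BeginPlay it reads the sheep total from BP_SheepSpawner, and its Box overlap events count BP_SheepFlocking actors entering and leaving.
; When the count reaches twice that total, likely because each sheep overlaps twice, it swaps all widgets for WBP_End_Flocking and shows the mouse cursor.
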(event `self.ReceiveBeginPlay`
  (bind _returnvalue (`GameplayStatics.GetActorOfClass` "/Game/Blueprint/BP_Flocking/BP_SheepSpawner.BP_SheepSpawner_C"))
  (bind _asbp_sheep_spawner (cast `/Game/Blueprint/BP_Flocking/BP_SheepSpawner` _returnvalue))
  (set `self.totalSheepCount` (`SheepSpawner.NumberOfSheepToSpawn` _asbp_sheep_spawner))
  (`KismetSystemLibrary.PrintText` (`KismetTextLibrary.Conv_IntToText` (`self.totalSheepCount`))))

(event `self.ReceiveTick`
  (params (DeltaSeconds :type "Float (single-precision)")))

(event `self.Box.OnComponentBeginOverlap`
  (params (OverlappedComponent :type "PrimitiveComponent Object Reference") (OtherActor :type "Actor Object Reference") (OtherComp :type "PrimitiveComponent Object Reference") (OtherBodyIndex :type Integer) (bFromSweep :type Boolean) (SweepResult :type "HitResult Structure (by ref)"))
  (cast `/Game/Blueprint/BP_Flocking/BP_SheepFlocking` OtherActor)
  (set `self.SheepInEnclosure` (+ (`self.SheepInEnclosure`) 1))
  (if (>= (`self.SheepInEnclosure`) (* (`self.totalSheepCount`) 2))
    (`KismetSystemLibrary.PrintText` "gagner !")
    (`WidgetLayoutLibrary.RemoveAllWidgets`)
    (bind _returnvalue (`|CreateWidget` "/Game/UI/WBP_End_Flocking.WBP_End_Flocking_C"))
    (`UserWidget.AddToViewport` _returnvalue 0)
    (set `PlayerController.bShowMouseCursor` true (`GameplayStatics.GetPlayerController` 0))
    (else
      (`KismetSystemLibrary.PrintText` (`KismetTextLibrary.Conv_IntToText` (`self.SheepInEnclosure`))))))

(event `self.Box.OnComponentEndOverlap`
  (params (OverlappedComponent :type "PrimitiveComponent Object Reference") (OtherActor :type "Actor Object Reference") (OtherComp :type "PrimitiveComponent Object Reference") (OtherBodyIndex :type Integer))
  (cast `/Game/Blueprint/BP_Flocking/BP_SheepFlocking` OtherActor)
  (set `self.SheepInEnclosure` (- (`self.SheepInEnclosure`) 1))
  (`KismetSystemLibrary.PrintText` (`KismetTextLibrary.Conv_IntToText` (`self.SheepInEnclosure`))))

(fn `UserConstructionScript`)